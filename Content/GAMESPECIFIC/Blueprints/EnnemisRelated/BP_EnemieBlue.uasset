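; Blue enemy actor that reacts to hits and fires bullets once struck.
; HitBlue starts a looping one-second Shoot timer and recomputes HP as damage minus current HP, using a third of the damage unless it is red.
; Each hit briefly swaps the mesh material before restoring blue, then calls Die if HP is zero or below.
; Shoot spawns short-lived BP_BulletE projectiles at the Scene component's transform.
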(event Custom|Shoot
  (bind _scene (Variables|Default|GetScene))
  (bind _returnvalue (Transformation|GetWorldTransform _scene))
  (bind _returnvalue_2 (Game|SpawnActorfromClass "/Game/GAMESPECIFIC/Blueprints/BP_BulletE.BP_BulletE_C" (Math|Transform|MakeTransform (.location _returnvalue) (.rotation _returnvalue) "1.000000,1.000000,1.000000") "Undefined" "MultiplyWithRoot" 0 0))
  (Actor|SetLifeSpan _returnvalue_2 1.0))

(event EventBeginPlay
  (|CallParentFunction) ; This node is disabled and will not be called.\nDrag off pins to build functionality.
)

(event Collision|EventActorBeginOverlap
  (params (OtherActor :type Actor%20Object%20Reference)))

(event EventTick
  (params (DeltaSeconds :type Float%20%28single-precision%29)))

(event EventHitBlue
  (params (dammage :type Integer) (redDammage :type Boolean))
  (Utilities|Time|SetTimerbyEvent (delegate Custom|Shoot) 1.0 true)
  (if redDammage
    (Variables|Default|SetHP (- dammage (Variables|Default|GetHP)))
    (else
      (Variables|Default|SetHP (- (/ dammage 3) (Variables|Default|GetHP)))))
  (Rendering|Material|SetMaterial (Variables|Character|GetMesh) 0 "/Game/GAMESPECIFIC/Materials/M_Master_Inst.M_Master_Inst")
  (Utilities|FlowControl|Delay 0.1)
  (Rendering|Material|SetMaterial (Variables|Character|GetMesh) 0 "/Engine/EngineDebugMaterials/VertexColorViewMode_BlueOnly.VertexColorViewMode_BlueOnly")
  (if (<= (Variables|Default|GetHP) 0)
    (CallFunction|Die)))

(fn ConstructionScript
  (|CallParentFunction))