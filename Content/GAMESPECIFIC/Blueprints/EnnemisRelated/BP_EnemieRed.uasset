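; BP_EnemieRed is a red enemy that reacts to hits through its HitRed event and dies when HP reaches zero or below.
; HitRed uses full damage for red hits and a third for others, setting HP to that amount minus current HP, rather than the reverse.
; Each hit briefly swaps the mesh material as a flash, then restores the red-only material before the HP check calls Die.
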(event EventBeginPlay
  (|CallParentFunction) ; This node is disabled and will not be called.\nDrag off pins to build functionality.
)

(event Collision|EventActorBeginOverlap
  (params (OtherActor :type Actor%20Object%20Reference)))

(event EventTick
  (params (DeltaSeconds :type Float%20%28single-precision%29)))

(event EventHitRed
  (params (dammage :type Integer) (redDammage :type Boolean))
  (if redDammage
    (Variables|Default|SetHP (- dammage (Variables|Default|GetHP)))
    (else
      (Variables|Default|SetHP (- (/ dammage 3) (Variables|Default|GetHP)))))
  (Rendering|Material|SetMaterial (Variables|Character|GetMesh) 0 "/Game/GAMESPECIFIC/Materials/M_Master_Inst1.M_Master_Inst1")
  (Utilities|FlowControl|Delay 0.1)
  (Rendering|Material|SetMaterial (Variables|Character|GetMesh) 0 "/Engine/EngineDebugMaterials/VertexColorViewMode_RedOnly.VertexColorViewMode_RedOnly")
  (if (<= (Variables|Default|GetHP) 0)
    (CallFunction|Die)))

(fn ConstructionScript
  (|CallParentFunction))