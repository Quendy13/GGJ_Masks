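; BP_Enemie is an enemy that endlessly chases the player's BP_TopDownCharacter and drops loot on death.
; BeginPlay caches the player, then AI MoveTo loops by calling ChaseAgain on success or failure.
; The die event randomly spawns low or high XP, then possibly a bronze or silver coin, at the capsule's location.
; As wired, the actor is destroyed only when a coin drops.
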(event Custom|die
  (bind _returnvalue (Math|Random|RandomIntegerinRange 0 10))
  (bind _capsulecomponent (Variables|Collision|GetCapsuleComponent))
  (bind _returnvalue_2 (Transformation|GetWorldLocation _capsulecomponent))
  ;[0.15 0.15 0.15 0.5] drop des ennemies fait de manière très brut a revoir mais foncionnelle
  (if (< (Math|Random|RandomIntegerinRange 0 10) 9)
    (Game|SpawnActorfromClass "/Game/GAMESPECIFIC/Blueprints/LevelRelated/Collectibles/BP_XPLow.BP_XPLow_C" (Math|Transform|MakeTransform _returnvalue_2 "0, 0, 0" "1.000000,1.000000,1.000000") "Undefined" "MultiplyWithRoot" 0 0)
    (else
      (Game|SpawnActorfromClass "/Game/GAMESPECIFIC/Blueprints/LevelRelated/Collectibles/BP_XPHigh.BP_XPHigh_C" (Math|Transform|MakeTransform _returnvalue_2 "0, 0, 0" "1.000000,1.000000,1.000000") "Undefined" "MultiplyWithRoot" 0 0)))
  (if (< _returnvalue 3)
    (Game|SpawnActorfromClass "/Game/GAMESPECIFIC/Blueprints/LevelRelated/Collectibles/BP_piècesBronze.BP_piècesBronze_C" (Math|Transform|MakeTransform (Transformation|GetWorldLocation (Variables|Collision|GetCapsuleComponent)) "0, 0, 0" "1.000000,1.000000,1.000000") "Undefined" "MultiplyWithRoot" 0 0)
    (Actor|DestroyActor :!label _label)
    (elif (< _returnvalue 4)
      (Game|SpawnActorfromClass "/Game/GAMESPECIFIC/Blueprints/LevelRelated/Collectibles/BP_piecesArgent.BP_piecesArgent_C" (Math|Transform|MakeTransform (Transformation|GetWorldLocation (Variables|Collision|GetCapsuleComponent)) "0, 0, 0" "1.000000,1.000000,1.000000") "Undefined" "MultiplyWithRoot" 0 0)
      (goto _label))))

(event Custom|ChaseAgain
  ;[0 0 0 0.5] Chasse le joueur peut importe l'endroit ou il se situe
  (AI|AIMoveTo self (.location (Transformation|GetActorTransform (stale EventBeginPlay _asbp_top_down_character))) (stale EventBeginPlay _asbp_top_down_character) 1e+01 false
    (:OnSuccess
      _)
    (:OnFail
      _))
  (CallFunction|ChaseAgain))

(event EventBeginPlay
  ;[0 0 0 0.5] Chasse le joueur peut importe l'endroit ou il se situe
  (bind _asbp_top_down_character (Utilities|Casting|CastToBP_TopDownCharacter (Game|Player|GetPlayerPawn 0)))
  (AI|AIMoveTo self (.location (Transformation|GetActorTransform _asbp_top_down_character)) _asbp_top_down_character 1e+01 false
    (:OnSuccess
      _)
    (:OnFail
      _))
  (CallFunction|ChaseAgain))

(fn ConstructionScript)