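; Blue bullet projectile that moves in a straight step-by-step path and deals blue-type damage to actors it overlaps.
; BeginPlay starts a very fast looping timer that offsets the Cube's world location by Direction without sweeping, then stores the result in CurrentLocation.
; Box overlap sends HitBlueMessage to the other actor with fixed damage and the red flag off.
; The graph never destroys the bullet, on hit or otherwise.
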(event OnComponentBeginOverlap(Box)
  (params (OverlappedComponent :type Primitive%20Component%20Object%20Reference) (OtherActor :type Actor%20Object%20Reference) (OtherComp :type Primitive%20Component%20Object%20Reference) (OtherBodyIndex :type Integer) (bFromSweep :type Boolean) (SweepResult :type Hit%20Result%20Structure%20%28by%20ref%29))
  (Class|BPIBulletInterface|HitBlue(Message) OtherActor 25 false))

(event Custom|forward
  (Transformation|SetWorldLocation (Variables|Default|Getcube) (+ (Variables|Default|Getcurrent%20location) (Variables|Default|Getdirection)) false false)
  (Variables|Default|Setcurrent%20location (Transformation|GetWorldLocation (Variables|Default|Getcube))))

(event EventBeginPlay
  (Utilities|Time|SetTimerbyEvent (delegate Custom|forward) 0.001 true))

(event Collision|EventActorBeginOverlap
  (params (OtherActor :type Actor%20Object%20Reference)))

(event EventTick
  (params (DeltaSeconds :type Float%20%28single-precision%29)))

(fn ConstructionScript)