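; BP_GameManager is a level manager that continuously spawns blue and red enemies around the player.
; On BeginPlay it starts two looping timers, each with its own interval, one per enemy type.
; Each tick spawns its enemy class at a random reachable navmesh point within a shared radius of the top-down character, adjusting for collision but always spawning.
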(event Custom|BP_EnemieRouge
  (Game|SpawnActorfromClass "/Game/GAMESPECIFIC/Blueprints/EnnemisRelated/BP_EnemieRed.BP_EnemieRed_C" (Math|Transform|MakeTransform (.RandomLocation (AI|Navigation|GetRandomReachablePointinRadius (Transformation|GetActorLocation (.AsBP%20Top%20Down%20Character (Utilities|Casting|CastToBP_TopDownCharacter (Game|Player|GetPlayerPawn 0)))) (Variables|Default|GetRadius) 0 0)) "0, 0, 0" "1.000000,1.000000,1.000000") "AdjustIfPossibleButAlwaysSpawn" "MultiplyWithRoot" 0 0))

(event Custom|EnemieBlue
  ;[0 0 0 0.5] Spawn des Enemies toutes les x secondes
  (Game|SpawnActorfromClass "/Game/GAMESPECIFIC/Blueprints/EnnemisRelated/BP_EnemieBlue.BP_EnemieBlue_C" (Math|Transform|MakeTransform (.RandomLocation (AI|Navigation|GetRandomReachablePointinRadius (Transformation|GetActorLocation (.AsBP%20Top%20Down%20Character (Utilities|Casting|CastToBP_TopDownCharacter (Game|Player|GetPlayerPawn 0)))) (Variables|Default|GetRadius) 0 0)) "0, 0, 0" "1.000000,1.000000,1.000000") "AdjustIfPossibleButAlwaysSpawn" "MultiplyWithRoot" 0 0))

(event EventBeginPlay
  ;[0 0 0 0.5] Spawn des Enemies toutes les x secondes
  (Utilities|Time|SetTimerbyEvent (delegate Custom|EnemieBlue) (Variables|Default|GetTimeB) true)
  (Utilities|Time|SetTimerbyEvent (delegate Custom|BP_EnemieRouge) (Variables|Default|GetTimeR) true))

(fn ConstructionScript)