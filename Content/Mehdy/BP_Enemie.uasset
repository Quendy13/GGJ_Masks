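; BP_Enemie is an enemy pawn that endlessly chases the top-down player character while shooting.
; BeginPlay starts a looping one-second timer for Shoot, then caches the player and begins the chase.
; AI MoveTo re-triggers through ChaseAgain on both success and failure, keeping pursuit going.
; Shoot spawns a short-lived BP_BulletE at the Scene component's location and rotation, independently of movement.
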(event Custom|Shoot
  (bind _scene (Variables|Default|GetScene))
  (bind _returnvalue (Transformation|GetWorldTransform _scene))
  ;[0 0 0 0.5] Chasse le joueur peut importe l'endroit ou il se situe
  (bind _returnvalue_2 (Game|SpawnActorfromClass "/Game/Mehdy/BP_BulletE.BP_BulletE_C" (Math|Transform|MakeTransform (.location _returnvalue) (.rotation _returnvalue) "1.000000,1.000000,1.000000") "Undefined" "MultiplyWithRoot" 0 0))
  (Actor|SetLifeSpan _returnvalue_2 1.0))

(event Custom|ChaseAgain
  ;[0 0 0 0.5] Chasse le joueur peut importe l'endroit ou il se situe
  (AI|AIMoveTo self (.location (Transformation|GetActorTransform (stale EventBeginPlay _asbp_top_down_character))) (stale EventBeginPlay _asbp_top_down_character) 1e+01 false
    (:OnSuccess
      _)
    (:OnFail
      _))
  (CallFunction|ChaseAgain))

(event EventBeginPlay
  ;[0 0 0 0.5] Chasse le joueur peut importe l'endroit ou il se situe
  (Utilities|Time|SetTimerbyEvent (delegate Custom|Shoot) 1.0 true)
  (bind _asbp_top_down_character (Utilities|Casting|CastToBP_TopDownCharacter (Game|Player|GetPlayerPawn 0)))
  (AI|AIMoveTo self (.location (Transformation|GetActorTransform _asbp_top_down_character)) _asbp_top_down_character 1e+01 false
    (:OnSuccess
      _)
    (:OnFail
      _))
  (CallFunction|ChaseAgain))

(fn ConstructionScript)