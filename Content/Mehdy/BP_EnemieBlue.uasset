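; Blue enemy that chases the player pawn and fires bullets.
; BeginPlay starts a looping timer that spawns BP_BulletE from an arrow component, and repeatedly re-issues AIMoveTo toward the player using Range as acceptance radius, one second after each success or failure.
; Hit subtracts health, cutting red damage to a third, then either calls Die or flashes the material and sets a Niagara burst.
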(event Custom|Shoot
  (bind _arrow1 (Variables|Default|GetArrow1))
  (bind _returnvalue (Transformation|GetWorldTransform _arrow1))
  (Game|SpawnActorfromClass "/Game/Mehdy/BP_BulletE.BP_BulletE_C" (Math|Transform|MakeTransform (.location _returnvalue) (.rotation _returnvalue) "1.000000,1.000000,1.000000") "Undefined" "MultiplyWithRoot" 0 0))

(event EventBeginPlay
  (Utilities|Time|SetTimerbyEvent (delegate Custom|Shoot) (Variables|Default|GetMinCD) true)
  ;[0 0 0 0.5] Zone de range bleu
  (bind _asbp_top_down_character (Utilities|Casting|CastToBP_TopDownCharacter (Game|Player|GetPlayerPawn 0) :!label _label))
  (AI|AIMoveTo self "0, 0, 0" _asbp_top_down_character (Variables|Default|Getrange) false
    (:OnSuccess
      _)
    (:OnFail
      _))
  (Utilities|FlowControl|Delay 1.0)
  (goto _label))

(event EventHit
  (params (dammage :type Integer) (redDammage :type Boolean))
  ;[0 0 0 0.5] Fait perdre de la vie sur le PNJ + tire projectile + die / feed back
  (if (not redDammage)
    (Variables|Default|SetHP_Bleu (- (Variables|Default|GetHP_Bleu) dammage))
    (else
      (Variables|Default|SetHP_Bleu (- (Variables|Default|GetHP_Bleu) (/ dammage 3)))))
  (if (<= (Variables|Default|GetHP_Bleu) 0)
    (CallFunction|Die)
    (else
      (Rendering|Material|SetMaterial (Variables|Character|GetMesh) 0 "/Game/Mehdy/Material/M_Master_Inst.M_Master_Inst")
      (Utilities|FlowControl|Delay 0.1)
      (Rendering|Material|SetMaterial (Variables|Character|GetMesh) 0 0)
      (Class|NiagaraComponent|SetAsset (Variables|Default|GetNiagara) "/Game/Pack_Simple_Particle_Burst/01_Niagara_Systems/NS_Simple_Burst_Level_1.NS_Simple_Burst_Level_1" true))))

(fn ConstructionScript
  (|CallParentFunction))